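; Grabbable map actor for the player's Sedan that shows the target NPC's position through a widget.
; GrabL and GrabR input attach the map's Billboard to the Sedan's left or right sphere, keeping world transform, when that sphere overlaps the Box; there is no release logic.
; Every Tick it searches all NPC_BP actors for those flagged as Target and writes their location into the Map_Widget's TargetPosition.
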(event `self.ReceiveBeginPlay`
  (`self.EnableInput` (`GameplayStatics.GetPlayerController` 0)))

(event `InputAction|GrabL` :consume false
  (params (Key :type "Key Structure" :default "AnyKey"))
  (:`Pressed`
    (bind _assedan (cast `/Game/VehicleBP/Sedan/Sedan` (`GameplayStatics.GetPlayerPawn` 0)))
    (bind _spherel (`/Game/VehicleBP/Sedan/Sedan.SphereL` _assedan))
    (if (`PrimitiveComponent.IsOverlappingComponent` (`self.Box`) _spherel)
      (`SceneComponent.K2_AttachToComponent` (`self.Billboard`) _spherel "None" "KeepWorld" "KeepWorld" "KeepWorld" true))))

(event `InputAction|GrabR` :consume false
  (params (Key :type "Key Structure" :default "AnyKey"))
  (:`Pressed`
    (bind _assedan (cast `/Game/VehicleBP/Sedan/Sedan` (`GameplayStatics.GetPlayerPawn` 0)))
    (bind _spherer (`/Game/VehicleBP/Sedan/Sedan.SphereR` _assedan))
    (if (`PrimitiveComponent.IsOverlappingComponent` (`self.Box`) _spherer)
      (`SceneComponent.K2_AttachToComponent` (`self.Billboard`) _spherer "None" "KeepWorld" "KeepWorld" "KeepWorld" true))))

(event `self.ReceiveTick`
  (params (DeltaSeconds :type "Float (single-precision)"))
  (bind _outactors (`GameplayStatics.GetAllActorsOfClass` "/Game/NPCs/NPC_BP.NPC_BP_C"))
  (for _array_element _outactors
    (if (== true (`/Game/NPCs/NPC_BP.Target` _array_element))
      (bind _asmap_widget (cast `/Game/Vehicle/Map_Widget` (`WidgetComponent.GetUserWidgetObject` (`self.Widget`))))
      (set `/Game/Vehicle/Map_Widget.TargetPosition` (`self.K2_GetActorLocation` _array_element) _asmap_widget))))

(fn `UserConstructionScript`)